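; BP_AnimalSpawner is an interactable spawner with a door and a fox visual mesh that spawns an animal when used.
; On BeginPlay, the visual mesh loops one fox idle or resting animation picked at random.
; Interact calls SpawnWAnim, which swings the door's yaw through a timeline in the DoorAnim graph, then calls SpawnAnimal once it finishes.
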(event `SpawnWAnim`
  (bind (_direction _zrotationvalue) (`Timeline|CustomAnimation`)
    (:`Update`
      (`SceneComponent.K2_SetRelativeRotation` (`self.Door`) (`KismetMathLibrary.MakeRotator` 0.0 0.0 _zrotationvalue) false false))
    (:`Finished`
      (`self.SpawnAnimal` "Move"))))

(event `self.ReceiveBeginPlay`
  (`self.PlayAnimationOnVisualMesh` "/Game/Animal/Fox/Animations/ANIM_Fox_IdleBreathe.ANIM_Fox_IdleBreathe" "/Game/Animal/Fox/Animations/ANIM_Fox_IdleLookAround.ANIM_Fox_IdleLookAround" "/Game/Animal/Fox/Animations/ANIM_Fox_Resting.ANIM_Fox_Resting" true))

(event `InteractionInterface.Interact`
  (params (InteractedActor :type "Actor Object Reference"))
  ;[1 1 1] Spawn Fox
  (`self.SpawnWAnim`))

(fn `PlayAnimationOnVisualMesh`
  (params (FirstAnimation :type "AnimationAsset Object Reference") (SecondAnimation :type "AnimationAsset Object Reference") (ThirdAnimation :type "AnimationAsset Object Reference") (bLooping :type Boolean))
  (`SkeletalMeshComponent.PlayAnimation` (`self.VisualMesh`) (`KismetArrayLibrary.Array_Random` (`|MakeArray` FirstAnimation SecondAnimation ThirdAnimation)) bLooping))

(fn `UserConstructionScript`)